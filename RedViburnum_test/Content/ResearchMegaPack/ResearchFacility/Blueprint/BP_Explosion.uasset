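; BP_Explosion is an overlap-triggered explosive with a breakable geometry collection that hurts the player character.
; When anything overlaps its Box, it applies an upward-biased impulse to the geometry collection, then after a short delay spawns a particle burst and sound at the actor.
; A BP_ThirdPersonCharacter overlapper takes fixed damage, and the actor destroys itself shortly afterward.
; Other overlappers fail the cast, leaving the actor in place.
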(event OnComponentBeginOverlap(Box)
  (params (OverlappedComponent :type Primitive%20Component%20Object%20Reference) (OtherActor :type Actor%20Object%20Reference) (OtherComp :type Primitive%20Component%20Object%20Reference) (OtherBodyIndex :type Integer) (bFromSweep :type Boolean) (SweepResult :type Hit%20Result%20Structure%20%28by%20ref%29))
  (bind _returnvalue (Transformation|GetActorLocation))
  (Physics|AddImpulse (Variables|Default|GetGeometryCollectionComponent) "10000.000000,10000.000000,40000.000000" "None" false)
  (Utilities|FlowControl|Delay 0.1)
  (Effects|SpawnEmitteratLocation "/Game/StarterContent/Particles/P_Explosion.P_Explosion" _returnvalue "0, 0, 0" "2.000000,2.000000,2.000000")
  (Audio|PlaySoundatLocation "/Game/StarterContent/Audio/Explosion02.Explosion02" _returnvalue "0, 0, 0" 1.0 1.0 0.0 0 0 0 0)
  (bind _asbp_third_person_character (Utilities|Casting|CastToBP_ThirdPersonCharacter OtherActor))
  (Game|Damage|ApplyDamage _asbp_third_person_character 13.0 0 0)
  (Utilities|FlowControl|Delay 1.1)
  (Actor|DestroyActor (Components|GetOwner (Variables|Default|GetBox))))

(event EventBeginPlay)

(event Collision|EventActorBeginOverlap
  (params (OtherActor :type Actor%20Object%20Reference)))

(event EventTick
  (params (DeltaSeconds :type Float%20%28single-precision%29)))

(fn ConstructionScript)